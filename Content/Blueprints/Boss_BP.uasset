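; Boss actor that takes over the camera, attacks with a staff, and makes the player lose on contact with the staff or Sphere1.
; It loops a timed windup and slam into a timeline spin that gains revolutions and duration as BossHP in Crash_GI drops.
; Overlapping its Box during the spin launches the player, removes HP and squashes the body.
; At zero HP it flattens and opens the main menu.
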(event OnComponentBeginOverlap(Box)
  (params (OverlappedComponent :type Primitive%20Component%20Object%20Reference) (OtherActor :type Actor%20Object%20Reference) (OtherComp :type Primitive%20Component%20Object%20Reference) (OtherBodyIndex :type Integer) (bFromSweep :type Boolean) (SweepResult :type Hit%20Result%20Structure%20%28by%20ref%29))
  ;[1 1 1] Hurt Animation
  (if (Variables|Default|GetCan%20Be%20Hurt)
    (Audio|Components|Audio|Stop (Variables|Default|GetSpin%20Timeline))
    (bind _asbp_third_person_character (Utilities|Casting|CastToBP_ThirdPersonCharacter OtherActor))
    (Character|LaunchCharacter _asbp_third_person_character "0.000000,0.000000,800.000000" false true)
    (Variables|Default|SetCan%20Be%20Hurt false)
    (Math|Integer|DecrementInt (Variables|/Game/Blueprints/Crash_GI.Crash_GI_C|GetBossHP (stale EventBeginPlay _ascrash_gi))
      (:%20%20
        (bind _float (Timeline|Hurt%20Timeline PlayFromStart)
          (:Update
            (Transformation|SetWorldScale3D (Variables|Default|GetBody) (Math|Vector|Lerp(Vector) "1.000000,1.000000,1.000000" "2.000000,2.000000,0.500000" _float)))
          (:Finished
            (if (> (Variables|/Game/Blueprints/Crash_GI.Crash_GI_C|GetBossHP (stale EventBeginPlay _ascrash_gi)) 0)
              (Variables|Default|SetRotation%20offset (.yaw (Transformation|GetWorldRotation (Variables|Default|GetBody))))
              (CallFunction|Windup)
              (else
                (CallFunction|Death)))))))))

(event OnComponentHit(Staff)
  (params (HitComponent :type Primitive%20Component%20Object%20Reference) (OtherActor :type Actor%20Object%20Reference) (OtherComp :type Primitive%20Component%20Object%20Reference) (NormalImpulse :type Vector :default "0, 0, 0") (Hit :type Hit%20Result%20Structure%20%28by%20ref%29))
  (bind _asbp_third_person_character (Utilities|Casting|CastToBP_ThirdPersonCharacter OtherActor))
  (Default|Lose _asbp_third_person_character))

(event OnComponentHit(Sphere1)
  (params (HitComponent :type Primitive%20Component%20Object%20Reference) (OtherActor :type Actor%20Object%20Reference) (OtherComp :type Primitive%20Component%20Object%20Reference) (NormalImpulse :type Vector :default "0, 0, 0") (Hit :type Hit%20Result%20Structure%20%28by%20ref%29))
  (bind _asbp_third_person_character (Utilities|Casting|CastToBP_ThirdPersonCharacter OtherActor))
  (Default|Lose _asbp_third_person_character))

(event Custom|Windup
  (bind _staff_slam (Variables|Default|GetStaff%20Slam))
  (bind _staff_windup (Variables|Default|GetStaff%20Windup))
  (bind _staff (Variables|Default|GetStaff))
  (Components|MoveComponentTo _staff (Variables|/Script/Engine.SceneComponent|GetRelativeLocation _staff_windup) (Variables|/Script/Engine.SceneComponent|GetRelativeRotation _staff_windup) false false 1.0 true)
  (Components|MoveComponentTo _staff (Variables|/Script/Engine.SceneComponent|GetRelativeLocation _staff_slam) (Variables|/Script/Engine.SceneComponent|GetRelativeRotation _staff_slam) false false 0.3 false)
  (CallFunction|Spin))

(event Custom|Spin
  (Variables|Default|SetCan%20Be%20Hurt true)
  (Utilities|FlowControl|Delay 0.5)
  (Components|Timeline|SetPlayRate (Variables|Default|GetSpin%20Timeline) (/ 1.0 (- 6 (Variables|/Game/Blueprints/Crash_GI.Crash_GI_C|GetBossHP (stale EventBeginPlay _ascrash_gi)))))
  (bind _newtrack_0 (Timeline|Spin%20Timeline PlayFromStart)
    (:Update
      (Transformation|SetWorldRotation (Variables|Default|GetBody) (Math|Rotator|MakeRotator 0.0 0.0 (Math|Float|Lerp (Variables|Default|GetRotation%20offset) (+ (Math|Conversions|ToFloat(Integer) (* (- 6 (Variables|/Game/Blueprints/Crash_GI.Crash_GI_C|GetBossHP (stale EventBeginPlay _ascrash_gi))) 360)) (Variables|Default|GetRotation%20offset)) _newtrack_0)) false false))
    (:Finished
      (Utilities|FlowControl|Delay 0.5)
      (Variables|Default|SetCan%20Be%20Hurt false)
      (CallFunction|Windup))))

(event Custom|Death
  (Components|DestroyComponent (Variables|Default|GetStaff))
  (bind _newtrack_0 (Timeline|Destroy%20Timeline Play)
    (:Update
      (Transformation|SetWorldScale3D (Variables|Default|GetBody) (Math|Vector|Lerp(Vector) "1.000000,1.000000,1.000000" "3.000000,3.000000,0.100000" _newtrack_0))
      (Utilities|FlowControl|Delay 5.0)
      (Game|OpenLevel(byObjectReference) "/Game/Levels/MainMenu.MainMenu"))))

(event EventBeginPlay
  (bind _ascrash_gi (Utilities|Casting|CastToCrash_GI (Game|GetGameInstance)))
  (Variables|/Game/Blueprints/Crash_GI.Crash_GI_C|SetisBoss _ascrash_gi true)
  (Game|Player|SetViewTargetwithBlend (Game|GetPlayerController 0) self 1.0 "VTBlend_Linear" 0.0 false)
  (CallFunction|Windup))

(fn ConstructionScript)