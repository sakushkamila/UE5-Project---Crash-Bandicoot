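; Fire trap actor that cycles a fire particle effect on and off on an endless timed loop.
; From BeginPlay, chained delays produce a pause, a brief warning-length burst, a second pause and a longer burst before looping back.
; The particle scale is set to the same unit value around the long burst, and the graph contains no damage or collision logic.
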(event EventBeginPlay
  (Components|Activation|Deactivate (Variables|Default|GetParticleSystem) :!label _label)
  (Utilities|FlowControl|Delay 2.0)
  (Components|Activation|Activate (Variables|Default|GetParticleSystem) false)
  (Utilities|FlowControl|Delay 0.2)
  (Components|Activation|Deactivate (Variables|Default|GetParticleSystem))
  (Utilities|FlowControl|Delay 1.0)
  (Components|Activation|Activate (Variables|Default|GetParticleSystem) false)
  (Transformation|SetWorldScale3D (Variables|Default|GetParticleSystem) "1.000000,1.000000,1.000000")
  (Utilities|FlowControl|Delay 1.0)
  (Transformation|SetWorldScale3D (Variables|Default|GetParticleSystem) "1.000000,1.000000,1.000000")
  (goto _label))

(fn ConstructionScript)