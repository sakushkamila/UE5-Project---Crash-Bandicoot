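; Base collectible actor that fires an empty ActionOnCollect event and destroys itself when a BP_ThirdPersonCharacter overlaps its sphere.
; An optional spawn timeline moves the sphere's relative Z, then hands over to an idle timeline that drives the same axis.
; A Gate controls pickup, opening at once when ImmediateCollect is set or there is no spawn animation, otherwise when the spawn animation finishes.
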(event OnComponentBeginOverlap(Sphere)
  (params (OverlappedComponent :type Primitive%20Component%20Object%20Reference) (OtherActor :type Actor%20Object%20Reference) (OtherComp :type Primitive%20Component%20Object%20Reference) (OtherBodyIndex :type Integer) (bFromSweep :type Boolean) (SweepResult :type Hit%20Result%20Structure%20%28by%20ref%29))
  (Utilities|Casting|CastToBP_ThirdPersonCharacter OtherActor)
  (Utilities|FlowControl|Gate true
    (:Exit
      (CallFunction|ActiononCollect)
      (Actor|DestroyActor))))

(event Custom|start%20idle%20animation
  (bind _z_coord (Timeline|Idle%20Timeline PlayFromStart)
    (:Update
      (Transformation|SetRelativeLocation (Variables|Default|GetSphere) (Math|Vector|MakeVector 0.0 0.0 _z_coord) false false))))

(event Custom|Action%20on%20Collect)

(event EventBeginPlay
  (if (Variables|Default|GetSpawnAnimation)
    (if (Variables|Default|GetImmediateCollect)
      (Utilities|FlowControl|Sequence
        (:then_0
          (Utilities|FlowControl|Gate true) ; enters at Open
        )
        (:then_1
          (bind _z_coord (Timeline|Spawn%20Timeline PlayFromStart)
            (:Update
              (Transformation|SetRelativeLocation (Variables|Default|GetSphere) (Math|Vector|MakeVector 0.0 0.0 _z_coord) false false))
            (:Finished
              (CallFunction|StartIdleAnimation)
              (Utilities|FlowControl|Gate true) ; enters at Open
            ))))
      (else
        (Timeline|Spawn%20Timeline PlayFromStart)))
    (else
      (CallFunction|StartIdleAnimation)
      (Utilities|FlowControl|Gate true) ; enters at Open
    )))

(fn ConstructionScript)