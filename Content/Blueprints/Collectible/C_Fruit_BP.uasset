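; C_Fruit_BP is a fruit collectible that adds to the player's fruit count when collected.
; Its ActiononCollect event casts the game instance to Crash_GI and increments FruitCnt.
; BeginPlay and the construction script only call the parent, and the file contains no overlap or pickup detection logic of its own.
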(event EventBeginPlay
  (|CallParentFunction))

(event Collision|EventActorBeginOverlap
  (params (OtherActor :type Actor%20Object%20Reference))
  (|CallParentFunction OtherActor) ; This node is disabled and will not be called.\nDrag off pins to build functionality.
)

(event EventTick
  (params (DeltaSeconds :type Float%20%28single-precision%29))
  (|CallParentFunction DeltaSeconds) ; This node is disabled and will not be called.\nDrag off pins to build functionality.
)

(event EventActiononCollect
  (bind _ascrash_gi (Utilities|Casting|CastToCrash_GI (Game|GetGameInstance)))
  (Math|Integer|IncrementInt (Variables|/Game/Blueprints/Crash_GI.Crash_GI_C|GetFruitCnt _ascrash_gi)))

(fn ConstructionScript
  (|CallParentFunction))