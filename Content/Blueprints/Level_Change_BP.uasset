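; Level-exit actor that either advances level progression or, when flagged Bonus, moves the player between a level and its bonus level.
; Overlapping the sphere opens the next level or MainMenu after the last; bonus portals require three keys.
; Crash_GI holds indices, keys and checkpoint state, letting BeginPlay place a returning player on the bonus portal with its collision disabled.
; The construction script picks the cylinder material from the Bonus flag.
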(event OnComponentBeginOverlap(Sphere)
  (params (OverlappedComponent :type Primitive%20Component%20Object%20Reference) (OtherActor :type Actor%20Object%20Reference) (OtherComp :type Primitive%20Component%20Object%20Reference) (OtherBodyIndex :type Integer) (bFromSweep :type Boolean) (SweepResult :type Hit%20Result%20Structure%20%28by%20ref%29))
  (if (Variables|Default|GetBonus)
    (bind _ascrash_gi (Utilities|Casting|CastToCrash_GI (Game|GetGameInstance)))
    (if (== (Variables|/Game/Blueprints/Crash_GI.Crash_GI_C|GetBonusKeys _ascrash_gi) 3)
      (CallFunction|LoadBonusLevel))
    (else
      (CallFunction|LoadNextLevel))))

(event Custom|Load%20Next%20Level
  (Input|DisableInput (Game|Player|GetPlayerPawn 0) (Game|GetPlayerController 0))
  (Utilities|FlowControl|Delay 0.2)
  (bind _ascrash_gi (Utilities|Casting|CastToCrash_GI (Game|GetGameInstance)))
  (bind _result (Math|Integer|IncrementInt (Variables|/Game/Blueprints/Crash_GI.Crash_GI_C|GetCurrentLevelIndex _ascrash_gi))
    (:%20%20
      (if (< _result (Utilities|Array|Length (Variables|/Game/Blueprints/Crash_GI.Crash_GI_C|GetLevel%20Progression%20 _ascrash_gi)))
        (Game|OpenLevel(byName) (Utilities|Array|Get(acopy) (Variables|/Game/Blueprints/Crash_GI.Crash_GI_C|GetLevel%20Progression%20 _ascrash_gi) _result))
        (else
          (Game|OpenLevel(byObjectReference) "/Game/Levels/MainMenu.MainMenu"))))))

(event Custom|Load%20Bonus%20Level
  (Input|DisableInput (Game|Player|GetPlayerPawn 0) (Game|GetPlayerController 0))
  (Utilities|FlowControl|Delay 0.2)
  (bind _ascrash_gi (Utilities|Casting|CastToCrash_GI (Game|GetGameInstance)))
  (if (Variables|/Game/Blueprints/Crash_GI.Crash_GI_C|GetInBonusLevel _ascrash_gi)
    (Variables|/Game/Blueprints/Crash_GI.Crash_GI_C|SetInBonusLevel _ascrash_gi false)
    (Game|OpenLevel(byName) (Utilities|Array|Get(acopy) (Variables|/Game/Blueprints/Crash_GI.Crash_GI_C|GetLevel%20Progression%20 _ascrash_gi) (Variables|/Game/Blueprints/Crash_GI.Crash_GI_C|GetCurrentLevelIndex _ascrash_gi)))
    (else
      (Variables|/Game/Blueprints/Crash_GI.Crash_GI_C|SetInBonusLevel _ascrash_gi true)
      (Variables|/Game/Blueprints/Crash_GI.Crash_GI_C|SetBonus%20Checkpoint%20Activated _ascrash_gi true)
      (Variables|/Game/Blueprints/Crash_GI.Crash_GI_C|SetBonus%20Checkpoint%20Location _ascrash_gi (Transformation|GetActorLocation))
      (Variables|/Game/Blueprints/Crash_GI.Crash_GI_C|SetBonusKeys _ascrash_gi 0)
      (Game|OpenLevel(byName) (Utilities|Array|Get(acopy) (Variables|/Game/Blueprints/Crash_GI.Crash_GI_C|GetBonus%20Levels _ascrash_gi) (Variables|/Game/Blueprints/Crash_GI.Crash_GI_C|GetCurrentLevelIndex _ascrash_gi))))))

(event EventBeginPlay
  (bind _ascrash_gi (Utilities|Casting|CastToCrash_GI (Game|GetGameInstance)))
  (if (Math|Boolean|ANDBoolean (Variables|/Game/Blueprints/Crash_GI.Crash_GI_C|GetBonus%20Checkpoint%20Activated _ascrash_gi) (not (Variables|/Game/Blueprints/Crash_GI.Crash_GI_C|GetInBonusLevel _ascrash_gi)) (Variables|Default|GetBonus))
    (Collision|SetCollisionEnabled (Variables|Default|GetSphere) "NoCollision")
    (Transformation|SetActorLocation (Game|Player|GetPlayerPawn 0) (+ (Transformation|GetActorLocation) "0.000000,0.000000,20.000000") false false)
    (Variables|/Game/Blueprints/Crash_GI.Crash_GI_C|SetBonus%20Checkpoint%20Activated _ascrash_gi false)))

(fn ConstructionScript
  (Rendering|Material|SetMaterial (Variables|Default|GetCylinder) 0 (select (Variables|Default|GetBonus) "/Game/StarterContent/Materials/M_CobbleStone_Rough.M_CobbleStone_Rough" "/Game/StarterContent/Materials/M_Tech_Hex_Tile_Pulse.M_Tech_Hex_Tile_Pulse")))