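; AkuAku_BP is an actor that moves once in a straight line from its placed location to the world position of its Endpoint component.
; On BeginPlay it caches both points and plays a Timeline whose alpha lerps the actor's location, without sweep.
; The Timeline play rate is derived from distance over Speed, so travel time scales with path length.
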(event EventBeginPlay
  (Variables|Default|SetFinish (Transformation|GetWorldLocation (Variables|Default|GetEndpoint)))
  (Variables|Default|SetStart (Transformation|GetActorLocation))
  (Components|Timeline|SetPlayRate (Variables|Default|GetTimeline) (/ 1.0 (/ (Math|Vector|VectorLength (- (Variables|Default|GetFinish) (Variables|Default|GetStart))) (Variables|Default|GetSpeed))))
  (bind _float (Timeline|Timeline Play)
    (:Update
      (Transformation|SetActorLocation (Math|Vector|Lerp(Vector) (Variables|Default|GetStart) (Variables|Default|GetFinish) _float) false false))))

(fn ConstructionScript)