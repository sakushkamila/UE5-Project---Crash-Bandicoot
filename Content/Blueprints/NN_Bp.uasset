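; Looping crusher trap that calls Lose on any BP_ThirdPersonCharacter overlapping its Box.
; Hit lerps the actor from Cube toward a point under Sphere at SpeedDown, then reverses at SpeedUp.
; After a pause, Shaking bobs it slightly along Z several times before triggering the next Hit.
; ChangeSpeed derives timeline play rates from travel distance and speed, keeping movement speed independent of distance.
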(event OnComponentBeginOverlap(Box)
  (params (OverlappedComponent :type Primitive%20Component%20Object%20Reference) (OtherActor :type Actor%20Object%20Reference) (OtherComp :type Primitive%20Component%20Object%20Reference) (OtherBodyIndex :type Integer) (bFromSweep :type Boolean) (SweepResult :type Hit%20Result%20Structure%20%28by%20ref%29))
  (bind _asbp_third_person_character (Utilities|Casting|CastToBP_ThirdPersonCharacter OtherActor))
  (Default|Lose _asbp_third_person_character))

(event Custom|change%20speed
  (params (NewParam :type Float%20%28double-precision%29))
  (Variables|Default|Setspeed NewParam)
  (Components|Timeline|SetPlayRate (Variables|Default|GetTimeline) (/ 1.0 (/ (Math|Vector|VectorLength (- (Variables|Default|Getstart) (Variables|Default|GetFinish))) (Variables|Default|Getspeed))))
  (Components|Timeline|SetPlayRate (Variables|Default|GetTimeline_0) (/ 1.0 (/ (Math|Vector|VectorLength (- (Variables|Default|Getstart) (Variables|Default|GetFinish))) (Variables|Default|Getspeed)))))

(event Custom|shaking
  (bind _cube (Variables|Components|GetCube))
  (bind _returnvalue (Transformation|GetWorldLocation _cube))
  (Variables|Default|SetIsDie false)
  (Variables|Default|SetStop 0)
  (Variables|Default|SetFinish (Math|Vector|MakeVector (.x _returnvalue) (.y _returnvalue) (+ (.z _returnvalue) 1e+01)))
  (Variables|Default|Setstart (Transformation|GetWorldLocation (Variables|Components|GetCube)))
  (CallFunction|ChangeSpeed (Variables|Default|Getspeed_down))
  (bind (_direction _float) (Timeline|Timeline_0 Play)
    (:Update
      (Transformation|SetActorLocation (Math|Vector|Lerp(Vector) (Variables|Default|Getstart) (Variables|Default|GetFinish) _float) false false))
    (:Finished
      (if (> (Variables|Default|GetStop) 4)
        (CallFunction|Hit)
        (else
          (Math|Integer|IncrementInt (Variables|Default|GetStop)
            (:%20%20
              (switch Utilities|FlowControl|Switch|SwitchonETimelineDirection _direction
                (:Forward
                  (Timeline|Timeline_0 ReverseFromEnd))
                (:Backward
                  (Timeline|Timeline_0 PlayFromStart))))))))))

(event Custom|hit
  (bind _sphere (Variables|Components|GetSphere))
  (bind _returnvalue (Transformation|GetWorldLocation _sphere))
  (Variables|Default|SetFinish (Math|Vector|MakeVector (.x _returnvalue) (.y _returnvalue) (- (.z _returnvalue) 47.0)))
  (Variables|Default|Setstart (Transformation|GetWorldLocation (Variables|Components|GetCube)))
  (CallFunction|ChangeSpeed (Variables|Default|Getspeed_down))
  (bind (_direction _float) (Timeline|Timeline Play)
    (:Update
      (Transformation|SetActorLocation (Math|Vector|Lerp(Vector) (Variables|Default|Getstart) (Variables|Default|GetFinish) _float) false false))
    (:Finished
      (Variables|Default|SetIsHit (Class|KismetMathLibrary|XORBoolean (Variables|Default|GetIsHit) true))
      (if (Variables|Default|GetIsHit)
        (CallFunction|ChangeSpeed (Variables|Default|Getspeed_up))
        (switch Utilities|FlowControl|Switch|SwitchonETimelineDirection _direction
          (:Forward
            (Timeline|Timeline ReverseFromEnd))
          (:Backward
            (Timeline|Timeline PlayFromStart)))
        (else
          (CallFunction|ChangeSpeed (Variables|Default|Getspeed_down))
          (Utilities|FlowControl|Delay 2.0)
          (CallFunction|Shaking))))))

(event EventBeginPlay
  (CallFunction|Hit))

(fn ConstructionScript)